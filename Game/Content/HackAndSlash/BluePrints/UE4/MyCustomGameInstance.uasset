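; Game instance for the HackAndSlash game that handles online sessions: searching, hosting, joining and destroying them.
; Search results are cached and pushed to the find-session menu, then matched by server name to join; direct IP joining uses an open console command.
; Hosting calls StartOnlineGame, shows the player controller's loading screen and opens TopDownExampleMap as a listen server.
; Travel and network errors are printed on screen.
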(event Custom|LoadingScreen_Event
  (bind _ashack_and_slash_player_controller (Utilities|Casting|CastToHackAndSlashPlayerController (Game|GetPlayerController 0)))
  (Class|HackandSlashPlayerController|LoadingScreen _ashack_and_slash_player_controller))

(event Custom|JoinIP_Event
  (Development|ExecuteConsoleCommand (Utilities|String|Append "open " (Variables|Default|GetIPToJoin)) (Game|GetPlayerController 0)))

(event Custom|JoinSession_Event
  (params (ServerName :type String))
  (for _array_element (Variables|Default|GetSessionResult)
    (if (Utilities|Enum|Equal(Enum) (Class|FindSessionsCallbackProxy|GetServerName _array_element) ServerName)
      (|JoinSession (Game|GetPlayerController 0) _array_element))))

(event Custom|SearchSession_Event
  (params (Find%20target :type Find%20Session%20Object%20Reference))
  (Variables|Default|SetFoundSessions 0)
  (bind _output_get (Variables|Default|SetFindSessionMenu Find%20target))
  (Default|RemoveServer _output_get)
  (Default|StartSearch _output_get)
  (bind _results (|FindSessions (Game|GetPlayerController 0) 100 false)
    (:then
      (Variables|Default|SetFoundSessions (+ (Variables|Default|GetFoundSessions) 1)))
    (:OnSuccess
      (Variables|Default|SetSessionResult _results)
      (if (!= (Variables|Default|GetFoundSessions) 0)
        (for _array_element (Variables|Default|GetSessionResult)
          (Default|ShowServer (Variables|Default|GetFindSessionMenu) _array_element)))
      (Default|EndSearch (Variables|Default|GetFindSessionMenu)))
    (:OnFailure
      (Default|EndSearch (Variables|Default|GetFindSessionMenu)))))

(event Custom|HostSession_Event
  (params (LAN :type Boolean) (Maxplayer :type Integer))
  (bind _returnvalue (Class|CustomGameInstance|StartOnlineGame "Coucou" LAN true Maxplayer))
  (if _returnvalue
    (CallFunction|LoadingScreenEvent)
    (Game|OpenLevel(byName) "TopDownExampleMap" true "listen")
    (else
      (Development|PrintString "Couldn't create session" true true "(R=1.000000,G=0.058392,B=0.000000,A=1.000000)"))))

(event Custom|DestroySession_Event
  (|DestroySession (Game|GetPlayerController 0)
    (:OnSuccess
      (Development|PrintString "Session destroyed"))
    (:OnFailure
      (Development|PrintString "Session destroyed failed"))))

(event EventHandleNetworkError
  (params (FailureType :type ENetworkFailure%20Enum :default "NetDriverAlreadyExists") (bIsServer :type Boolean))
  (Development|PrintString (Utilities|String|Append (Utilities|String|ToString(Byte) FailureType) (Utilities|String|Append " - is server: " (Utilities|String|ToString(Boolean) bIsServer)))))

(event EventHandleTravelError
  (params (FailureType :type ETravelFailure%20Enum :default "NoLevel"))
  (Development|PrintString (Utilities|String|EnumtoString FailureType)))