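; PlayerParty is an actor for a party character with a floating name label and life bar, highlighted through custom depth on cursor hover.
; Each tick it reloads the VideoSettings save and shows or hides both displays from its PlayerName and PlayerHealthBar flags.
; FaceCAmera also runs every tick, turning the name fully toward the player camera and the life bar on yaw only.
; A setplayername event fills the label text.
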(event Custom|setplayername_Event
  (params (Name :type String))
  (Rendering|Components|TextRender|SetText (Variables|Default|GetPlayerPartyName) (Utilities|Text|ToText(String) Name))
  (bind _returnvalue (SaveGame|DoesSaveGameExist "VideoSettings"))
  (if _returnvalue
    (bind _returnvalue_2 (SaveGame|LoadGamefromSlot "VideoSettings"))
    (bind _assetting_save (Utilities|Casting|CastToSettingSave _returnvalue_2))
    (Variables|Default|SetsaveGame _assetting_save)))

(event EventTick
  (params (DeltaSeconds :type Float%20%28single-precision%29))
  (bind _savegame (Variables|Default|GetSaveGame))
  (bind _playerpartyname (Variables|Default|GetPlayerPartyName))
  (bind _life (Variables|Default|GetLife))
  (bind _savegame_2 (Variables|Default|GetSaveGame))
  (bind _returnvalue (Rendering|IsVisible _playerpartyname))
  (bind _returnvalue_2 (Rendering|IsVisible _life))
  (Utilities|FlowControl|Sequence
    (:then_0
      (bind _returnvalue_3 (SaveGame|DoesSaveGameExist "VideoSettings"))
      (if _returnvalue_3
        (bind _returnvalue_4 (SaveGame|LoadGamefromSlot "VideoSettings"))
        (bind _assetting_save (Utilities|Casting|CastToSettingSave _returnvalue_4))
        (Variables|Default|SetsaveGame _assetting_save)))
    (:then_1
      (CallFunction|FaceCAmera))
    (:then_2
      (Utilities|IsValid _savegame_2
        (:Is%20Valid
          (if (Variables|/Game/HackAndSlash/Interface/Option/SettingSave.SettingSave_C|GetPlayerName _savegame_2)
            (if (not _returnvalue)
              (Rendering|SetVisibility _playerpartyname true false))
            (elif _returnvalue
              (Rendering|SetVisibility _playerpartyname false false))))))
    (:then_3
      (Utilities|IsValid _savegame
        (:Is%20Valid
          (if (Variables|/Game/HackAndSlash/Interface/Option/SettingSave.SettingSave_C|GetPlayerHealthBar _savegame)
            (if (not _returnvalue_2)
              (Rendering|SetVisibility _life true false))
            (elif _returnvalue_2
              (Rendering|SetVisibility _life false false))))))))

(event MouseInput|EventActorBeginCursorOver
  (Rendering|SetRenderCustomDepth (Variables|Character|GetMesh) true))

(event MouseInput|EventActorEndCursorOver
  (Rendering|SetRenderCustomDepth (Variables|Character|GetMesh) false))

(fn ConstructionScript)

(fn FaceCAmera
  (bind _playerpartyname (Variables|Default|GetPlayerPartyName))
  (bind _life (Variables|Default|GetLife))
  (Utilities|IsValid (Game|GetPlayerCameraManager 0)
    (:Is%20Valid
      (Transformation|SetWorldRotation _playerpartyname (Math|Rotator|FindLookatRotation (Transformation|GetWorldLocation _playerpartyname) (Transformation|GetActorLocation (Game|GetPlayerCameraManager 0))) false false)
      (Transformation|SetWorldRotation _life (Math|Rotator|MakeRotator 0.0 0.0 (.Yaw (Math|Rotator|BreakRotator (Math|Rotator|FindLookatRotation (Transformation|GetWorldLocation _life) (Transformation|GetActorLocation (Game|GetPlayerCameraManager 0)))))) false false))))