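; Player controller for an online hack-and-slash, bridging the MyClient network actor with UI and pawns.
; Marker actors identify the map as game, menu or character creation, choosing between spawning a TopDownCharacter with HUD and opening the matching widget.
; Client callbacks drive login, friends, group invites, popups, level entry and spawned PlayerParty proxies for teammates.
; In game, gated click-to-move uses SimpleMoveToLocation and reports position with a map ID.
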(event Custom|SpawnCharacterMenuCreate
  (params (Class :type Class%20Enum))
  ;[1 1 1] Spawn character menu create
  (bind _outactors (Actor|GetAllActorsOfClass "/Game/InfinityBladeWarriors/Character/CompleteCharacters/CreatePlrBp.CreatePlrBp_C"))
  (Variables|Default|SetPlayerCreated (Utilities|Array|Get(acopy) _outactors))
  (switch Utilities|FlowControl|Switch|SwitchonClass Class
    (:NewEnumerator0
      (Variables|Default|SetPlayerCreateSelection "/Game/InfinityBladeWarriors/Character/CompleteCharacters/SK_CharM_Barbarous.SK_CharM_Barbarous"))
    (:NewEnumerator1
      (Variables|Default|SetPlayerCreateSelection "/Game/InfinityBladeWarriors/Character/CompleteCharacters/SK_CharM_Shell.SK_CharM_Shell"))
    (:NewEnumerator2
      (Variables|Default|SetPlayerCreateSelection "/Game/InfinityBladeWarriors/Character/CompleteCharacters/SK_CharM_Robo.SK_CharM_Robo"))
    (:NewEnumerator3
      (Variables|Default|SetPlayerCreateSelection "/Game/InfinityBladeWarriors/Character/CompleteCharacters/SK_CharM_Forge.SK_CharM_Forge"))
    (:NewEnumerator4
      (Variables|Default|SetPlayerCreateSelection "/Game/InfinityBladeWarriors/Character/CompleteCharacters/SK_CharM_Tusk.SK_CharM_Tusk")))
  (Class|SkinnedMeshComponent|SetSkeletalMesh (Variables|/Script/Engine.Character|GetMesh (Variables|Default|GetPlayerCreated)) (Variables|Default|GetPlayerCreateSelection)))

(event Custom|BackToMenu
  ;[1 1 1] Back to menu
  (bind _outactors (Actor|GetAllActorsOfClass "/Game/HackAndSlash/BluePrints/GAme/MyClient.MyClient_C"))
  (Class|Client|ReturntoMenu (Utilities|Array|Get(acopy) _outactors))
  (if (Variables|Default|GetisInGame)
    (bind _returnvalue (UserInterface|CreateWidget "/Game/HackAndSlash/Interface/Menu/WaitTimer.WaitTimer_C"))
    (UserInterface|Viewport|AddtoViewport _returnvalue 0)
    (Utilities|FlowControl|Delay 5.0)
    (Game|OpenLevel(byName) "MenuMaps")
    (else
      (Game|OpenLevel(byName) "MenuMaps"))))

(event Custom|PreEnterInGame
  (params (DesiredMap :type String))
  ;[1 1 1] Pré enter in game
  (bind _mapid (CallFunction|GetMapID DesiredMap))
  (bind _outactors (Actor|GetAllActorsOfClass "/Game/HackAndSlash/BluePrints/GAme/MyClient.MyClient_C"))
  (Utilities|IsValid (Utilities|Array|Get(acopy) _outactors)
    (:Is%20Valid
      (Class|Client|SendEnterWorldReq (Utilities|Array|Get(acopy) _outactors) _mapid))))

(event Custom|Spawn_Event
  (params (Controller :type Player%20Controller%20Object%20Reference))
  ;[1 1 1] Spawn
  (Networking|SwitchHasAuthority
    (:Authority
      (bind _outactors (Actor|GetAllActorsOfClass "/Script/Engine.PlayerStart"))
      (Utilities|IsValid (Utilities|Array|Get(acopy) _outactors (Math|Random|RandomIntegerinRange 0 (- (Utilities|Array|Length _outactors) 1)))
        (:Is%20Valid
          (bind _returnvalue (Game|SpawnActorfromClass "/Game/TopDownCPP/Blueprints/TopDownCharacter.TopDownCharacter_C" (Transformation|GetActorTransform (Utilities|Array|Get(acopy) _outactors (Math|Random|RandomIntegerinRange 0 (- (Utilities|Array|Length _outactors) 1)))) "Undefined" self 0))
          (Utilities|FlowControl|Delay 1.0)
          (Pawn|Possess Controller _returnvalue)
          (bind _returnvalue_2 (UserInterface|CreateWidget "/Game/HackAndSlash/Interface/Game/HUD.HUD_C" (Game|GetPlayerController 0)))
          (UserInterface|Viewport|AddtoViewport _returnvalue_2 0)
          (Variables|Default|SetHUDS _returnvalue_2)
          (bind _outactors_2 (Actor|GetAllActorsOfClass "/Game/HackAndSlash/BluePrints/GAme/MyClient.MyClient_C"))
          (Utilities|IsValid (Utilities|Array|Get(acopy) _outactors_2)
            (:Is%20Valid
              (Class|HackandSlashPlayerController|RefreshMaps)
              (bind _returnvalue_3 (Game|GetCurrentLevelName true))
              (bind _mapid (CallFunction|GetMapID _returnvalue_3))
              (Class|Client|SendEnterWorldComplete (Utilities|Array|Get(acopy) _outactors_2) self (Transformation|GetActorLocation _returnvalue) _mapid)
              (bind _outactors_3 (Actor|GetAllActorsOfClass "/Game/HackAndSlash/BluePrints/GAme/MyClient.MyClient_C"))
              (Utilities|IsValid (Utilities|Array|Get(acopy) _outactors_3)
                (:Is%20Valid
                  (Class|Client|Init (Utilities|Array|Get(acopy) _outactors_3) self))))))))))

(event EventOnPopupMessageRes
  (params (TheMessage :type String))
  ;[1 1 1] Popup message
  (bind _returnvalue (UserInterface|CreateWidget "/Game/HackAndSlash/Interface/Game/AlerteMessage.AlerteMessage_C"))
  (Default|ChangeAlerteTextEvent _returnvalue TheMessage)
  (UserInterface|Viewport|AddtoViewport _returnvalue 0))

(event EventOnMapsListRecv
  (params (maps :type Array%20of%20Maps%20Structures))
  ;[1 1 1] Recv maps list
  (Variables|Default|SetMaps maps))

(event EventFriendNotificationResult
  (params (online :type Boolean) (NameOfFriend :type String))
  ;[1 1 1] Friend notification
  (bind _returnvalue (SaveGame|DoesSaveGameExist "VideoSettings"))
  (if _returnvalue
    (bind _returnvalue_2 (SaveGame|LoadGamefromSlot "VideoSettings"))
    (bind _assetting_save (Utilities|Casting|CastToSettingSave _returnvalue_2))
    (if (Variables|/Game/HackAndSlash/Interface/Option/SettingSave.SettingSave_C|GetFriendConnection _assetting_save)
      (bind _returnvalue_3 (UserInterface|CreateWidget "/Game/HackAndSlash/Interface/Game/Friend/FriendNotification.FriendNotification_C" :!label _label))
      (UserInterface|Viewport|AddtoViewport _returnvalue_3 0)
      (Default|SetInfosEvent _returnvalue_3 NameOfFriend online))
    (else
      (goto _label))))

(event EventFriendListResult
  (params (lists :type Array%20of%20Friend%20Structures))
  (bind _menu (Variables|Default|GetMenu))
  ;[1 1 1] Friend list result
  (Development|PrintString "On friend list result")
  (Utilities|IsValid _menu
    (:Is%20Valid
      (Development|PrintString "menu valid")
      (Default|OnFriendListRECVEvent _menu lists))))

(event EventMovePlayerParty
  (params (destination :type Vector) (charID :type Integer))
  ;[1 1 1] Move player party
  (bind _outactors (Actor|GetAllActorsOfClass "/Game/HackAndSlash/BluePrints/UE4/PlayerParty.PlayerParty_C"))
  (for _array_element _outactors
    (Utilities|IsValid _array_element
      (:Is%20Valid
        (if (== (Variables|/Game/HackAndSlash/BluePrints/UE4/PlayerParty.PlayerParty_C|GetcharID _array_element) charID)
          (AI|Navigation|SimpleMovetoLocation (Pawn|GetController _array_element) destination))))))

(event EventCharacterLoadResult
  (params (haveCharacter :type Boolean))
  ;[1 1 1] Character load result
)

(event EventOnGroupeInviteRecv
  (params (accountID :type Integer) (name :type String))
  ;[1 1 1] Groupe invite Recv
  (bind _returnvalue (UserInterface|CreateWidget "/Game/HackAndSlash/Interface/Game/Friend/friendInviteRecv.friendInviteRecv_C"))
  (UserInterface|Viewport|AddtoViewport _returnvalue 0)
  (Variables|/Game/HackAndSlash/Interface/Game/Friend/friendInviteRecv.friendInviteRecv_C|SetaccountID _returnvalue accountID)
  (Rendering|Components|TextRender|SetText (Variables|/Game/HackAndSlash/Interface/Game/Friend/friendInviteRecv.friendInviteRecv_C|Getname _returnvalue) (Utilities|Text|ToText(String) name)))

(event EventOnEnterGameRes
  (params (canEnter :type Boolean) (Levelname :type String))
  ;[1 1 1] On game enter res
  (if canEnter
    (Class|HackandSlashPlayerController|LoadingScreen)
    (Game|OpenLevel(byName) (Utilities|String|StringToName Levelname))))

(event EventLoginResult
  (params (LoginResult :type LoginResultEnum%20Enum :default "BadPassword"))
  (bind _menu (Variables|Default|GetMenu))
  ;[1 1 1] Login result
  (Utilities|IsValid _menu
    (:Is%20Valid
      (Default|LoggingResultEvent _menu LoginResult))))

(event EventSpawnPlayerParty
  (params (partyMember :type Spawn%20Friend%20Party%20Structure))
  (bind (_name _level _charid _location) (Utilities|Struct|BreakSpawnFriendParty partyMember))
  ;[1 1 1] Spawn player party
  (bind _returnvalue (Game|SpawnActorfromClass "/Game/HackAndSlash/BluePrints/UE4/PlayerParty.PlayerParty_C" (Math|Transform|MakeTransform _location) "AlwaysSpawn" 0 0))
  (bind _output_get (Variables|Default|SetotherPlayer _returnvalue))
  (Variables|/Game/HackAndSlash/BluePrints/UE4/PlayerParty.PlayerParty_C|SetcharID _output_get _charid)
  (Default|SetplayernameEvent _output_get _name)
  (Utilities|GetMapCheck
    (:Game
      (Default|AddPlayerGroupeFrameEvent (Variables|Default|GetHUDS) (Variables|Default|GetFriendList)))))

(event EventRemovePlayerParty
  (params (charID :type Integer))
  ;[1 1 1] Remove player party
  (bind _outactors (Actor|GetAllActorsOfClass "/Game/HackAndSlash/BluePrints/UE4/PlayerParty.PlayerParty_C"))
  (for _array_element _outactors
    (if (== (Variables|/Game/HackAndSlash/BluePrints/UE4/PlayerParty.PlayerParty_C|GetcharID _array_element) charID)
      (Actor|DestroyActor _array_element))))

(event EventOnRemoveGroupRecv
  ;[1 1 1] Refresh / Remove group
  (Utilities|GetMapCheck
    (:Game
      (Default|ClearGroupeEvent (Variables|Default|GetHUDS)))
    (:Menu
      (Default|RemoveFriendGroupEvent (Variables|Default|GetMenu)))))

(event EventOnRefreshGroupRecv
  (params (friends :type Array%20of%20Refresh%20Friend%20Structures))
  ;[1 1 1] Refresh / Remove group
  (Variables|Default|SetFriendList friends)
  (Utilities|GetMapCheck
    (:Game
      (Default|AddPlayerGroupeFrameEvent (Variables|Default|GetHUDS) (Variables|Default|GetFriendList)))
    (:Menu
      (Default|AddFriendGrouptoMenuEvent (Variables|Default|GetMenu) (Variables|Default|GetFriendList)))))

(event EventTick
  (params (DeltaSeconds :type Float%20%28single-precision%29))
  (bind (_hitresult _returnvalue) (Game|Player|GetHitResultUnderCursorbyChannel "TraceTypeQuery1" true))
  ;[1 1 1] TICK
  (Utilities|FlowControl|Sequence
    (:then_0
      (if (Variables|Default|GetisInGame)
        (Utilities|FlowControl|Gate true ; While key is pressed...
          (:Exit
            (if _returnvalue
              (CallFunction|MovetoHitLocation _hitresult) ; ..and move there.
            )))))))

(event EventBeginPlay
  ;[1 1 1] BeginPlay
  (bind _outactors (Actor|GetAllActorsOfClass "/Game/HackAndSlash/BluePrints/GAme/MyClient.MyClient_C"))
  (Utilities|IsValid (Utilities|Array|Get(acopy) _outactors)
    (:Is%20Valid
      (Utilities|GetMapCheck
        (:Game
          (Variables|Default|SetisInGame true)
          (Pawn|UnPossess)
          (if (Pawn|IsLocalPlayerController)
            (CallFunction|SpawnEvent self)))
        (:Menu
          (if (Pawn|IsLocalPlayerController)
            (CallFunction|OnMenuCreate)))
        (:Character
          (if (Pawn|IsLocalPlayerController)
            (bind _returnvalue (UserInterface|CreateWidget "/Game/HackAndSlash/Interface/CharacterCreate/CreateCharacter.CreateCharacter_C" (Game|GetPlayerController 0)))
            (UserInterface|Viewport|AddtoViewport _returnvalue 0)))))))

(event Input|ActionEvents|InputActionEchape
  (params (Key :type Key%20Structure :default "AnyKey"))
  ;[1 1 1] Escape
  (:Pressed
    (Utilities|IsValid (Variables|Default|GetEscapeMenu)
      (:Is%20Valid
        (switch Utilities|FlowControl|Switch|SwitchonESlateVisibility (Widget|GetVisibility (Variables|Default|GetEscapeMenu))
          (:Visible
            (Widget|SetVisibility (Variables|Default|GetEscapeMenu) "Hidden"))
          (:Hidden
            (Widget|SetVisibility (Variables|Default|GetEscapeMenu) "Visible"))))
      (:Is%20Not%20Valid
        (bind _returnvalue (UserInterface|CreateWidget "/Game/HackAndSlash/Interface/Menu/EscapeMenu.EscapeMenu_C"))
        (bind _output_get (Variables|Default|SetEscapeMenu _returnvalue))
        (UserInterface|Viewport|AddtoViewport _output_get 0)))))

(event Input|ActionEvents|InputActionSetDestination
  (params (Key :type Key%20Structure :default "AnyKey"))
  (bind _returnvalue (Game|GetPlayerController 0))
  (bind (_hitresult _returnvalue_2) (Game|Player|GetHitResultUnderCursorbyChannel "TraceTypeQuery1" true))
  (bind _isingame (Variables|Default|GetisInGame))
  (bind (_worldlocation _worlddirection) (Game|Player|ConvertMouseLocationToWorldSpace _returnvalue))
  ;[1 1 1] TICK
  (:Pressed
    (if _isingame
      (Utilities|FlowControl|Gate true) ; enters at Open
    ))
  (:Released
    (if _isingame
      (CallFunction|MovetoHitLocation (.HitResult (Game|Player|GetHitResultUnderCursorbyChannel "TraceTypeQuery1" true))) ; ..and move there.
      (bind _outhit (Collision|LineTraceByChannel _worldlocation (* (+ (Math|Vector|GetForwardVector (Pawn|GetControlRotation _returnvalue :!class /Script/Engine.Controller)) 1.2e+04) _worlddirection) "TraceTypeQuery2" false 0 "None"))
      (Effects|SpawnEmitteratLocation "/Game/InfinityBlade/Effect/Effects/FX_Ambient/UI_MainMenu/P_UserDestination.P_UserDestination" (Math|Vector|MakeVector (.X (Math|Vector|BreakVector (.Location (Collision|BreakHitResult _outhit)))) (.Y (Math|Vector|BreakVector (.Location (Collision|BreakHitResult _outhit)))) (+ (.Z (Math|Vector|BreakVector (.Location (Collision|BreakHitResult _outhit)))) 5.0)) "0.000000,0.000000, 0")
      (Utilities|FlowControl|Gate true) ; enters at Close
    )))

(fn ConstructionScript)

(fn GetMapID
  (params (DesiredMap :type String))
  (for _array_element (Variables|Default|GetMaps)
    (if (Utilities|Enum|Equal(Enum) (.name (Utilities|Struct|BreakMaps _array_element)) DesiredMap)
      (LocalVariables|SetmapsID (.id (Utilities|Struct|BreakMaps _array_element)))))
  (return (LocalVariables|GetmapsID)))

(fn OnMenuCreate
  (bind _outactors (Actor|GetAllActorsOfClass "/Game/HackAndSlash/BluePrints/GAme/MyClient.MyClient_C"))
  (Utilities|IsValid (Utilities|Array|Get(acopy) _outactors)
    (:Is%20Valid
      (bind _output_get (LocalVariables|SetMyClientPointer (Utilities|Array|Get(acopy) _outactors)))
      (bind _returnvalue (UserInterface|CreateWidget "/Game/HackAndSlash/Interface/Menu/Menu.Menu_C" (Game|GetPlayerController 0)))
      (UserInterface|Viewport|AddtoViewport _returnvalue 0)
      (Variables|Default|SetMenu _returnvalue)
      (bind _returnvalue_2 (Class|Client|IsAlreadyInitialized (LocalVariables|GetMyClientPointer)))
      (if _returnvalue_2
        _
        (else
          (Class|Client|Init _output_get (.AsMy%20Custom%20Character%20Controller (Utilities|Casting|CastToMyCustomCharacterController (Game|GetPlayerController 0))))))
      (bind _returnvalue_3 (Class|Client|IsConnected (LocalVariables|GetMyClientPointer)))
      (if _returnvalue_3
        (Default|ConstructInitializedEvent (Variables|Default|GetMenu))
        (else
          (Default|ConstructDefaultEvent (Variables|Default|GetMenu)))))))

(fn MovetoHitLocation
  (params (Hit :type Hit%20Result%20Structure))
  (bind _location (Collision|BreakHitResult Hit))
  (if (>= (Math|Vector|VectorLength (- (Transformation|GetActorLocation (Pawn|GetControlledPawn)) _location)) (Variables|Default|GetMinClickDistance)) ; Don't move if player clicks too close to pawn
    (AI|Navigation|SimpleMovetoLocation self _location) ; Send the destination point to the character
    (bind _returnvalue (Game|GetCurrentLevelName true))
    (bind _mapid (CallFunction|GetMapID _returnvalue))
    (Class|HackandSlashPlayerController|UpadtePosition _location _mapid)))